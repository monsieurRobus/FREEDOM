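; Third-person player Character that handles movement, camera look and ownership of an inventory.
; On BeginPlay it spawns a Bp_Inventory actor with a slot grid layout, passing itself as owner reference, and stores the result.
; Axis inputs move it relative to control yaw and rotate the controller.
; Actions trigger jump and crouch, while holding "run" lowers max walk speed and releasing raises it.
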(event `self.ReceiveBeginPlay`
  ;[1 1 1] Spawn Inventory
  (bind _returnvalue (`|SpawnActorFromClass` "/Game/InventorySystem/Blueprints/Bp_Inventory.Bp_Inventory_C" (`KismetMathLibrary.MakeTransform` (0.0 0.0 0.0)) "AlwaysSpawn" "OverrideRootScale" null 20 self 4))
  (set `self.InventoryRef` _returnvalue))

(event `InputAxis|MoveForward`
  (params (AxisValue :type "Float (single-precision)"))
  ;[1 1 1] Movement
  (`self.AddMovementInput` (`KismetMathLibrary.GetForwardVector` (`KismetMathLibrary.MakeRotator` 0.0 0.0 (.yaw (`self.GetControlRotation`)))) AxisValue))

(event `InputAxis|MoveRight`
  (params (AxisValue :type "Float (single-precision)"))
  ;[1 1 1] Movement
  (`self.AddMovementInput` (`KismetMathLibrary.GetRightVector` (`KismetMathLibrary.MakeRotator` 0.0 0.0 (.yaw (`self.GetControlRotation`)))) AxisValue))

(event `InputAxis|LookPitch`
  (params (AxisValue :type "Float (single-precision)"))
  ;[1 1 1] RotController
  (`self.AddControllerPitchInput` AxisValue))

(event `InputAction|Jump`
  (params (Key :type "Key Structure" :default "AnyKey"))
  ;[1 1 1] Crouch/Jump
  (:`Pressed`
    (`self.Jump`)))

(event `InputAction|run`
  (params (Key :type "Key Structure" :default "AnyKey"))
  (bind _charactermovement (`self.CharacterMovement`))
  ;[1 1 1] Run
  (:`Pressed`
    (set `CharacterMovementComponent.MaxWalkSpeed` 600.0 _charactermovement))
  (:`Released`
    (set `CharacterMovementComponent.MaxWalkSpeed` 900.0 _charactermovement)))

(event `InputAxis|LookYaw`
  (params (AxisValue :type "Float (single-precision)"))
  ;[1 1 1] RotController
  (`self.AddControllerYawInput` AxisValue))

(event `InputAction|Crouch`
  (params (Key :type "Key Structure" :default "AnyKey"))
  ;[1 1 1] Crouch/Jump
  (:`Pressed`
    (`self.Crouch`)))

(fn `UserConstructionScript`)